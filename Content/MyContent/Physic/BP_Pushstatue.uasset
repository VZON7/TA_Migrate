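; BP_Pushstatue is a statue actor that kicks up dust when the player pushes it.
; On a Box hit by player character 0 while the Box has non-zero velocity, it spawns NS_Dust attached to the Box, offset downward.
; Each qualifying hit spawns a new system and overwrites the DustParticle reference; the logic to deactivate it is unconnected and never runs.
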(event `self.Box.OnComponentHit`
  (params (HitComponent :type "PrimitiveComponent Object Reference") (OtherActor :type "Actor Object Reference") (OtherComp :type "PrimitiveComponent Object Reference") (NormalImpulse :type "Vector Structure") (Hit :type "HitResult Structure (by ref)"))
  (if (and (== (`GameplayStatics.GetPlayerCharacter` 0) OtherActor) (!= (`SceneComponent.GetComponentVelocity` (`self.Box`)) (0.0 0.0 0.0)))
    (bind _returnvalue (`NiagaraFunctionLibrary.SpawnSystemAttached` "/Game/MyContent/FX/Dust/NS_Dust.NS_Dust" (`self.Box`) "None" (0.0 0.0 -50.0) (struct) "KeepRelativeOffset"))
    (set `self.DustParticle` _returnvalue)))

(fn `UserConstructionScript`)