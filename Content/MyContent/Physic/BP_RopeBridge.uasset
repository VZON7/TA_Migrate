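; Rope bridge actor that builds a physics-driven chain of planks in its construction script, sized by PlankAmount.
; Plank meshes are spaced evenly along X with a randomly flipped rotation, and a physics constraint joins each neighboring pair at its midpoint.
; The first and last planks have physics disabled to act as anchors.
; The Cable component's end is moved to the last plank's X and given a rope material.
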(fn `AddConstraints`
  (bind _relativelocation_x (`KismetMathLibrary.BreakVector` (`SceneComponent.RelativeLocation` (`|GetArrayItem` (`self.Planks`) (`self.Index`)))))
  (for _index (range (`self.PlankAmount`))
    (set `self.Index` _index)
    (bind _returnvalue (`AddComponent|NODE_AddPhysicsConstraintComponent-0` :`RelativeTransform` (`KismetMathLibrary.MakeTransform` (`KismetMathLibrary.MakeVector` (+ _relativelocation_x 40.0)))))
    (`PhysicsConstraintComponent.SetConstrainedComponents` _returnvalue (`|GetArrayItem` (`self.Planks`) (`self.Index`)) "None" (`|GetArrayItem` (`self.Planks`) (+ (`self.Index`) 1)) "None")))

(fn `AddPlanks`
  (for _index (range (+ (`self.PlankAmount`) 1))
    (bind _returnvalue (`AddComponent|NODE_AddStaticMeshComponent-0` :`RelativeTransform` (`KismetMathLibrary.MakeTransform` (`KismetMathLibrary.MakeVector` (`KismetMathLibrary.Conv_IntToDouble` (* _index 80))) (select `int` (`KismetMathLibrary.RandomIntegerInRange` 0 1) :`0` (struct :`Yaw` 90.0) :`1` (struct :`Yaw` -90.0) :!type "Rotator Structure") (2.0 2.0 2.0))))
    (`KismetArrayLibrary.Array_Add` (`self.Planks`) _returnvalue)))

(fn `UserConstructionScript`
  (bind _planks (`self.Planks`))
  (bind _relativelocation_x (`KismetMathLibrary.BreakVector` (`SceneComponent.RelativeLocation` (`|GetArrayItem` _planks (`KismetArrayLibrary.Array_LastIndex` _planks)))))
  (`self.AddPlanks`)
  (`self.AddConstraints`)
  ;[0.3542 0.2779 0.149] 1st and last plank wont simulate physic even on sky
  (`PrimitiveComponent.SetSimulatePhysics` (`|GetArrayItem` (`self.Planks`)) false)
  (`PrimitiveComponent.SetSimulatePhysics` (`|GetArrayItem` _planks (`KismetArrayLibrary.Array_LastIndex` _planks)) false)
  ;[0.3707 0.8697 1] scale the cable
  (set `CableComponent.EndLocation` (`KismetMathLibrary.MakeVector` _relativelocation_x -140.0 110.0) (`self.Cable`))
  (`PrimitiveComponent.SetMaterial` (`self.Cable`) 0 "/Game/Megascans/Surfaces/Three_Strand_Manila_Rope_ulztacqs/MI_Three_Strand_Manila_Rope_ulztacqs_2K.MI_Three_Strand_Manila_Rope_ulztacqs_2K"))